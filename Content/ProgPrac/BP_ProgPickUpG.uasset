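; A score pickup whose cube moves vertically on a timeline, started at a random time offset on BeginPlay.
; When a BP_ThirdPersonCharacter overlaps its box, it adds a small random amount to the Score on the BP_ProgPrac actor found in the level.
; It then prints the new score to screen and destroys itself.
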(event `self.ReceiveBeginPlay`
  (`|ExecutionSequence`
    (:`then_0`
      (bind (_direction _newtrack_0) (`Timeline|Timeline` :`NewTime` (`KismetMathLibrary.RandomFloat`) :!via `SetNewTime` :!label _label)
        (:`Update`
          (`SceneComponent.K2_SetRelativeLocation` (`self.Cube`) (`KismetMathLibrary.VLerp` (0.0 0.0 125.0) (0.0 0.0 75.0) _newtrack_0) false false))))
    (:`then_1`
      (goto _label))))

(event `self.Box.OnComponentBeginOverlap`
  (params (OverlappedComponent :type "PrimitiveComponent Object Reference") (OtherActor :type "Actor Object Reference") (OtherComp :type "PrimitiveComponent Object Reference") (OtherBodyIndex :type Integer) (bFromSweep :type Boolean) (SweepResult :type "HitResult Structure (by ref)"))
  (cast `/Game/ThirdPerson/Blueprints/BP_ThirdPersonCharacter` OtherActor)
  (bind _returnvalue (`GameplayStatics.GetActorOfClass` "/Game/ProgPrac/BP_ProgPrac.BP_ProgPrac_C"))
  (bind _output_get (set `/Game/ProgPrac/BP_ProgPrac.Score` (+ (`/Game/ProgPrac/BP_ProgPrac.Score` _returnvalue) (`KismetMathLibrary.RandomIntegerInRange` 5 10)) _returnvalue))
  (`KismetSystemLibrary.PrintString` (`KismetStringLibrary.Conv_IntToString` _output_get) true true (struct :`R` 1.0 :`B` 0.012348 :`A` 1.0))
  (`self.K2_DestroyActor`))

(fn `UserConstructionScript`)