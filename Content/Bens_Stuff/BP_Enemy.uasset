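; BP_Enemy is a basic enemy Blueprint with a health value that takes damage and dies.
; A TakeDamage event subtracts the incoming amount from Health, and the CheckIfDead function tests whether it has reached zero or below to destroy the actor.
; It prints debug strings on BeginPlay and on each hit; the construction script is empty.
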(event `self.ReceiveBeginPlay`
  (`KismetSystemLibrary.PrintString` "Hello, Time to die!"))

(event `Take Damage`
  (params (`By amount` :type "Float (double-precision)"))
  (`KismetSystemLibrary.PrintString` "Pain")
  (set `self.Health` (- (`self.Health`) `By amount`))
  (if (`self.CheckIfDead` (`self.Health`))
    (`self.K2_DestroyActor`)))

(fn `CheckIfDead`
  (params (Health :type "Float (double-precision)"))
  (returns (IsDead :type Boolean))
  (return (<= Health 0.0)))

(fn `UserConstructionScript`)