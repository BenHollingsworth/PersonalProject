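; BP_EnemyTester is a test actor that repeatedly damages every BP_Enemy in the level.
; From BeginPlay it finds all BP_Enemy actors, prints their count, then calls TakeDamage on each with a small random amount while printing its index.
; After a completion message and a short delay, it calls its GiveDamage event again, looping indefinitely.
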(event `Give Damage`
  ;[1 1 1] Find all BP_Enemy
  (bind _outactors (`GameplayStatics.GetAllActorsOfClass` "/Game/Bens_Stuff/BP_Enemy.BP_Enemy_C" :!label _label))
  (`KismetSystemLibrary.PrintString` (`KismetStringLibrary.Concat_StrStr` "There are " (`KismetStringLibrary.Conv_IntToString` (`KismetArrayLibrary.Array_Length` _outactors)) " enemies in the level"))
  (for (_array_element _array_index) _outactors
    (`/Game/Bens_Stuff/BP_Enemy.Take Damage` _array_element (`KismetMathLibrary.RandomFloatInRange` 0.1 0.5))
    (`KismetSystemLibrary.PrintString` (`KismetStringLibrary.Concat_StrStr` "This is enemy " (`KismetStringLibrary.Conv_IntToString` _array_index))))
  (`KismetSystemLibrary.PrintString` "We've given damage to all of the enemies")
  (`KismetSystemLibrary.Delay` 2.0)
  (`self.Give Damage`))

(event `self.ReceiveBeginPlay`
  (goto _label))

(fn `UserConstructionScript`)