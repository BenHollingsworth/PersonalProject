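; BP_Item is a carryable item actor with pickup, drop and use events, the last only printing a debug message.
; Pickup disables the Cube's collision and snaps an attachment to the Item_Hand_Place socket using the passed-in capsule component.
; Drop detaches the Cube, restores collision and simulates physics for a brief delay before switching it off.
; The Cube is hidden on BeginPlay.
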(event `Pickup`
  (params (`Capsule Component ` :type "SceneComponent Object Reference"))
  (`KismetSystemLibrary.PrintString` "Picked up")
  ;[1 1 1] Don't push
  (`PrimitiveComponent.SetCollisionEnabled` (`self.Cube`) "NoCollision")
  (`self.K2_AttachToComponent` null "Item_Hand_Place" "SnapToTarget" "SnapToTarget" "KeepRelative")
  (`self.K2_AttachToComponent` `Capsule Component ` "Item_Hand_Place" "SnapToTarget" "SnapToTarget" "KeepRelative"))

(event `Drop`
  (`KismetSystemLibrary.PrintString` "Item dropped")
  (`SceneComponent.K2_DetachFromComponent` (`self.Cube`) "KeepWorld" "KeepWorld" "KeepRelative" false)
  (`PrimitiveComponent.SetCollisionEnabled` (`self.Cube`) "QueryAndPhysics")
  (`PrimitiveComponent.SetSimulatePhysics` (`self.Cube`) true)
  (`KismetSystemLibrary.Delay` 2.0)
  (`PrimitiveComponent.SetSimulatePhysics` (`self.Cube`) false))

(event `self.ReceiveBeginPlay`
  (`SceneComponent.SetVisibility` (`self.Cube`) false false))

(event `primaryAction`
  (params (HeldDown :type Boolean))
  (`KismetSystemLibrary.PrintString` "Item Used"))

(fn `UserConstructionScript`)