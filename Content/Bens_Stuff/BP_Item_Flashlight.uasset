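; Flashlight item Blueprint whose light shines only while the primary action is held down.
; The Flashlight component starts hidden on BeginPlay, and the PrimaryAction event shows or hides it from its HeldDown flag, printing a debug message for each state.
; The construction script only calls its parent version.
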(event `self.ReceiveBeginPlay`
  (`SceneComponent.SetVisibility` (`self.Flashlight`) false false))

(event `self.primaryAction`
  (params (HeldDown :type Boolean))
  (if HeldDown
    (`KismetSystemLibrary.PrintString` "Light is on")
    (`SceneComponent.SetVisibility` (`self.Flashlight`) true false)
    (else
      (`KismetSystemLibrary.PrintString` "Light is off")
      (`SceneComponent.SetVisibility` (`self.Flashlight`) false false))))

(fn `UserConstructionScript`
  (`parent.UserConstructionScript`))